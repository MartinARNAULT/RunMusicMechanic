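; BP_Character is a character with keyboard-driven movement along the world Y axis and a jump.
; D, A and Space Bar press and release events set movement booleans that Tick reads each frame.
; Tick applies unswept world offsets by CharacterSpeed, unscaled by delta time, bypassing movement input.
; Jumping is an instant Y and Z offset by JumpSize and JumpHeight, applied while Space is held and CharacterMovement is not falling.
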(event `self.ReceiveTick`
  (params (DeltaSeconds :type "Float (single-precision)"))
  (`|ExecutionSequence`
    (:`then_0`
      (if (`self.ForwardMove`)
        (`self.K2_AddActorWorldOffset` (`KismetMathLibrary.MakeVector` 0.0 (`self.CharacterSpeed`)))))
    (:`then_1`
      (if (`self.BackMove`)
        (`self.K2_AddActorWorldOffset` (`KismetMathLibrary.MakeVector` 0.0 (* (`self.CharacterSpeed`) -1.0)))))
    (:`then_2`
      (if (`NavMovementComponent.IsFalling` (`self.CharacterMovement`))
        _
        (elif (`self.JumpBool`)
          (`self.K2_AddActorWorldOffset` (`KismetMathLibrary.MakeVector` 0.0 (`self.JumpSize`) (`self.JumpHeight`))))))))

(event `Key|D`
  (params (Key :type "Key Structure"))
  ;[0 0.3153 1] Bool Movment
  (:`Pressed`
    (set `self.ForwardMove` true))
  (:`Released`
    (set `self.ForwardMove` false)))

(event `Key|A`
  (params (Key :type "Key Structure"))
  ;[0 0.3153 1] Bool Movment
  (:`Pressed`
    (set `self.BackMove` true))
  (:`Released`
    (set `self.BackMove` false)))

(event `Key|SpaceBar`
  (params (Key :type "Key Structure"))
  ;[0 0.3153 1] Bool Movment
  (:`Pressed`
    (set `self.JumpBool` true))
  (:`Released`
    (set `self.JumpBool` false)))

(fn `UserConstructionScript`)